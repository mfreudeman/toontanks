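; Base game mode Blueprint that drives the UI for a match against turrets, from start to win or loss.
; On game start it shows a start widget with the start delay and creates and stores the player HUD.
; Health and turret-count events update that HUD.
; Game over adds an end screen widget that receives whether the player won.
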(event `self.PlayerHealthUpdated`
  (params (CurrentHealth :type "Float (single-precision)") (MaxHealth :type "Float (single-precision)"))
  (`/Game/Blueprints/Widgets/WBP_HUD.SetHealth` (`self.PlayerHUD`) CurrentHealth MaxHealth))

(event `self.TurretCountChanged`
  (params (TurretsRemaining :type Integer))
  (`/Game/Blueprints/Widgets/WBP_HUD.SetTurretCount` (`self.PlayerHUD`) TurretsRemaining))

(event `self.GameStart`
  (bind _returnvalue (`|CreateWidget` "/Game/Blueprints/Widgets/WBP_GameStart.WBP_GameStart_C"))
  (`/Game/Blueprints/Widgets/WBP_GameStart.SetStartDelay` _returnvalue (`self.StartDelay`))
  (`UserWidget.AddToViewport` _returnvalue 0)
  (bind _returnvalue_2 (`|CreateWidget` "/Game/Blueprints/Widgets/WBP_HUD.WBP_HUD_C"))
  (`UserWidget.AddToViewport` _returnvalue_2 0)
  (set `self.PlayerHUD` _returnvalue_2))

(event `self.GameOver`
  (params (bPlayerWon :type Boolean))
  (bind _returnvalue (`|CreateWidget` "/Game/Blueprints/Widgets/WBP_GameEnd.WBP_GameEnd_C"))
  (`/Game/Blueprints/Widgets/WBP_GameEnd.SetPlayerWon` _returnvalue bPlayerWon)
  (`UserWidget.AddToViewport` _returnvalue 0))

(fn `UserConstructionScript`)